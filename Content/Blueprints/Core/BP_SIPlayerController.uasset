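; BP_SIPlayerController is the player controller that boots the player into the game's title menu and handles pausing.
; On BeginPlay it shows WBP_TitleMenu, plays the ambient main sound and registers the IMC_PlayerMain Enhanced Input mapping context.
; Completing the IA_Escape action creates a new WBP_PauseMenu and adds it to the player screen at Z-order 1.
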(event `self.ReceiveBeginPlay`
  (bind _returnvalue (`|CreateWidget` "/Game/Blueprints/UI/WBP_TitleMenu.WBP_TitleMenu_C" self))
  (`UserWidget.AddToPlayerScreen` _returnvalue 0)
  (`GameplayStatics.PlaySound2D` "/Game/Music/AmbientMain.AmbientMain" 1.0 1.0 0.0 null null)
  (`EnhancedInputSubsystemInterface.AddMappingContext` (pcsubsystem `EnhancedInputLocalPlayerSubsystem` self) "/Game/Input/IMC_PlayerMain.IMC_PlayerMain" 0 (struct)))

(event `EnhancedInput|/Game/Input/Actions/IA_Escape`
  (params (ActionValue :type Boolean) (ElapsedSeconds :type "Float (double-precision)") (TriggeredSeconds :type "Float (double-precision)") (InputAction :type "InputAction Object Reference" :default "/Game/Input/Actions/IA_Escape.IA_Escape"))
  (:`Completed`
    (bind _returnvalue (`|CreateWidget` "/Game/Blueprints/UI/WBP_PauseMenu.WBP_PauseMenu_C" self))
    (`UserWidget.AddToPlayerScreen` _returnvalue 1)))

(fn `UserConstructionScript`)