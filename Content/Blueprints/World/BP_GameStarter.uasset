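; BP_GameStarter is a trigger volume that starts the game when the player pawn enters it.
; On BeginPlay it registers with GlobalEventsManager as a GameStartVolume object.
; An overlap of Bounds by a BP_SIPlayerPawn calls StartGame on that manager.
; ShowObject and HideObject toggle the trigger's query collision along with the visibility of its box and text label.
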(event `self.ReceiveBeginPlay`
  (`GlobalEventsManager.RegisterGameObject` (subsystem `GlobalEventsManager`) self "GameStartVolume"))

(event `self.Bounds.OnComponentBeginOverlap`
  (params (OverlappedComponent :type "PrimitiveComponent Object Reference") (OtherActor :type "Actor Object Reference") (OtherComp :type "PrimitiveComponent Object Reference") (OtherBodyIndex :type Integer) (bFromSweep :type Boolean) (SweepResult :type "HitResult Structure (by ref)"))
  (cast `/Game/Blueprints/Core/BP_SIPlayerPawn` OtherActor)
  (`GlobalEventsManager.StartGame` (subsystem `GlobalEventsManager`)))

(event `self.ShowObject`
  (`PrimitiveComponent.SetCollisionEnabled` (`self.Bounds`) "QueryOnly")
  (`SceneComponent.SetHiddenInGame` (`self.BoxBounds`) false true)
  (`SceneComponent.SetHiddenInGame` (`self.TextRender`) false true))

(event `self.HideObject`
  (`PrimitiveComponent.SetCollisionEnabled` (`self.Bounds`) "NoCollision")
  (`SceneComponent.SetHiddenInGame` (`self.BoxBounds`) true true)
  (`SceneComponent.SetHiddenInGame` (`self.TextRender`) true true))

(fn `UserConstructionScript`)